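; BP_HandSlot is a hand slot actor that holds a card in a card game and snaps it back into place.
; On BeginPlay it scans all BP_CardParent actors, setting its IsInHand flag from each one's lock state and calling SetInHand for unlocked ones.
; Tick assigns the held card's OnReleased event every frame, re-snapping that card on release unless locked.
; SetInHand moves CardInPossession to the Cube's XY at a fixed height.
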(event Custom|OnReleased_Event
  (params (TouchedActor :type Actor%20Object%20Reference) (ButtonReleased :type Key%20Structure :default "None"))
  (if (not (Variables|/Game/Blueprint/Cards/BP_CardParent.BP_CardParent_C|GetIsLocked (Variables|Default|GetCardInPossession)))
    (CallFunction|SetinHand)))

(event EventBeginPlay
  (bind _outactors (Actor|GetAllActorsOfClass "/Game/Blueprint/Cards/BP_CardParent.BP_CardParent_C"))
  (for _array_element _outactors
    (if (Variables|/Game/Blueprint/Cards/BP_CardParent.BP_CardParent_C|GetIsLocked _array_element)
      (Variables|Default|SetIsInHand? false)
      (else
        (Variables|Default|SetIsInHand? true)
        (CallFunction|SetinHand)))))

(event Collision|EventActorBeginOverlap
  (params (OtherActor :type Actor%20Object%20Reference)))

(event EventTick
  (params (DeltaSeconds :type Float%20%28single-precision%29))
  (EventDispatchers|AssignOnReleased (Variables|Default|GetCardInPossession) (delegate Custom|OnReleased_Event)))

(fn ConstructionScript)

(fn SetinHand
  (bind _cube (Variables|Default|GetCube))
  (bind _returnvalue (Transformation|GetWorldLocation _cube))
  (Transformation|SetActorLocation (Variables|Default|GetCardInPossession) (Math|Vector|MakeVector (.x _returnvalue) (.y _returnvalue) 1e+01) false false))