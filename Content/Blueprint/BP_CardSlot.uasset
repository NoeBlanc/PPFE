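; Board slot for a card-capture game that holds one card and tracks whether the player or bot owns it.
; OnCardPlaced claims the slot for the player, then compares the card's edge values against occupied neighbour slots, capturing those it strictly beats.
; Tick locks owned cards and sets the slot material by owner, while BeginPlay snaps pre-placed bot cards onto the slot.
; Only the upward fight also updates the captured card's CardOwner.
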(event Custom|OnCardPlaced
  (params (CardPlaced :type BP%20Card%20Parent%20Object%20Reference))
  ;[1 1 1] Appelé par une carte lorsqu'elle est placée
  (bind _output_get (Variables|Default|SetCard%20Placed CardPlaced))
  (Variables|Default|SetIsOccupiedByPlayer true)
  (Variables|Default|SetIsOccupiedByBot false)
  (CallFunction|FightSlotUp _output_get)
  (CallFunction|FightSlotDown _output_get)
  (CallFunction|FightSlotLeft _output_get)
  (CallFunction|FightSlotRight _output_get))

(event EventTick
  (params (DeltaSeconds :type Float%20%28single-precision%29))
  (bind _card_placed (Variables|Default|GetCard%20Placed))
  (bind _card_placed_2 (Variables|Default|GetCard%20Placed))
  ;[1 1 1] Une fois que le système d'appartenance des cases est fait pour le montrer
  (if (Variables|Default|GetIsOccupiedByPlayer)
    (Variables|/Game/Blueprint/Cards/BP_CardParent.BP_CardParent_C|SetIsLocked _card_placed true)
    (Collision|SetCollisionResponsetoAllChannels (Variables|/Game/Blueprint/Cards/BP_CardParent.BP_CardParent_C|GetCube _card_placed) "ECR_Ignore")
    (Rendering|Material|SetMaterial (Variables|Default|GetSlot) 0 "/Game/StarterContent/Materials/M_Brick_Clay_Beveled.M_Brick_Clay_Beveled")
    (elif (Variables|Default|GetIsOccupiedByBot)
      (Variables|/Game/Blueprint/Cards/BP_CardParent.BP_CardParent_C|SetIsLocked _card_placed_2 true)
      (Collision|SetCollisionResponsetoAllChannels (Variables|/Game/Blueprint/Cards/BP_CardParent.BP_CardParent_C|GetCube _card_placed_2) "ECR_Ignore")
      (Rendering|Material|SetMaterial (Variables|Default|GetSlot) 0 "/Game/StarterContent/Materials/M_Concrete_Grime.M_Concrete_Grime")
      (Default|ShowStats _card_placed_2)
      (else
        (Rendering|Material|SetMaterial (Variables|Default|GetSlot) 0 "/Game/StarterContent/Materials/M_Basic_Wall.M_Basic_Wall")))))

(event EventBeginPlay
  (bind _card_placed (Variables|Default|GetCard%20Placed))
  (bind _slot (Variables|Default|GetSlot))
  (bind _returnvalue (Transformation|GetWorldLocation _slot))
  ;[1 1 1] Vérifie si une carte est déjà placée ou non
  (if (Variables|Default|GetIsOccupiedByBot)
    (if (Utilities|IsValid _card_placed)
      (Variables|/Game/Blueprint/Cards/BP_CardParent.BP_CardParent_C|SetIsLocked _card_placed true)
      (Transformation|SetActorLocation _card_placed (Math|Vector|MakeVector (.x _returnvalue) (.y _returnvalue) 1e+01) false false))))

(fn ConstructionScript)

(fn FightSlotUp
  (params (CardInfo :type BP%20Card%20Parent%20Object%20Reference))
  (bind _slotup (Variables|Default|GetSlotUp))
  (if (Utilities|IsValid (Variables|Default|GetSlotUp))
    (if (Utilities|IsValid (Variables|BP_CardSlot_C|GetCard%20Placed (Variables|Default|GetSlotUp)))
      (Development|PrintString "j'ai un slot occupé au dessus de moi" true true "(R=1.000000,G=0.102237,B=0.072390,A=1.000000)")
      (if (> (Variables|/Game/Blueprint/Cards/BP_CardParent.BP_CardParent_C|GetTopValue CardInfo) (Variables|/Game/Blueprint/Cards/BP_CardParent.BP_CardParent_C|GetBottomValue (Variables|BP_CardSlot_C|GetCard%20Placed (Variables|Default|GetSlotUp))))
        (Rendering|Material|SetMaterial (Variables|BP_CardSlot_C|GetSlot _slotup) 0 "/Game/Blueprint/Cards/CardsTexture/BowmanTexture.BowmanTexture")
        (Variables|BP_CardSlot_C|SetIsOccupiedByPlayer _slotup true)
        (bind _output_get (Variables|/Game/Blueprint/Cards/BP_CardParent.BP_CardParent_C|SetCardOwner (Variables|BP_CardSlot_C|GetCard%20Placed _slotup) "NewEnumerator0"))
        (Development|PrintString (Utilities|String|EnumtoString _output_get))
        (else
          (Variables|BP_CardSlot_C|SetIsOccupiedByBot _slotup true))))))

(fn FightSlotDown
  (params (CardInfo :type BP%20Card%20Parent%20Object%20Reference))
  (bind _slotdown (Variables|Default|GetSlotDown))
  (if (Utilities|IsValid (Variables|Default|GetSlotDown))
    (if (Utilities|IsValid (Variables|BP_CardSlot_C|GetCard%20Placed (Variables|Default|GetSlotDown)))
      (if (> (Variables|/Game/Blueprint/Cards/BP_CardParent.BP_CardParent_C|GetBottomValue CardInfo) (Variables|/Game/Blueprint/Cards/BP_CardParent.BP_CardParent_C|GetTopValue (Variables|BP_CardSlot_C|GetCard%20Placed (Variables|Default|GetSlotDown))))
        (Rendering|Material|SetMaterial (Variables|BP_CardSlot_C|GetSlot _slotdown) 0 "/Game/Blueprint/Cards/CardsTexture/BowmanTexture.BowmanTexture")
        (Variables|BP_CardSlot_C|SetIsOccupiedByPlayer _slotdown true)
        (else
          (Variables|BP_CardSlot_C|SetIsOccupiedByBot _slotdown true))))))

(fn FightSlotLeft
  (params (CardInfo :type BP%20Card%20Parent%20Object%20Reference))
  (bind _slotleft (Variables|Default|GetSlotLeft))
  (if (Utilities|IsValid (Variables|Default|GetSlotLeft))
    (if (Utilities|IsValid (Variables|BP_CardSlot_C|GetCard%20Placed (Variables|Default|GetSlotLeft)))
      (if (> (Variables|/Game/Blueprint/Cards/BP_CardParent.BP_CardParent_C|GetLeftValue CardInfo) (Variables|/Game/Blueprint/Cards/BP_CardParent.BP_CardParent_C|GetRightValue (Variables|BP_CardSlot_C|GetCard%20Placed (Variables|Default|GetSlotLeft))))
        (Rendering|Material|SetMaterial (Variables|BP_CardSlot_C|GetSlot _slotleft) 0 "/Game/Blueprint/Cards/CardsTexture/BowmanTexture.BowmanTexture")
        (Variables|BP_CardSlot_C|SetIsOccupiedByPlayer _slotleft true)
        (else
          (Variables|BP_CardSlot_C|SetIsOccupiedByBot _slotleft true))))))

(fn FightSlotRight
  (params (CardInfo :type BP%20Card%20Parent%20Object%20Reference))
  (bind _slotright (Variables|Default|GetSlotRight))
  (if (Utilities|IsValid (Variables|Default|GetSlotRight))
    (if (Utilities|IsValid (Variables|BP_CardSlot_C|GetCard%20Placed (Variables|Default|GetSlotRight)))
      (if (> (Variables|/Game/Blueprint/Cards/BP_CardParent.BP_CardParent_C|GetRightValue CardInfo) (Variables|/Game/Blueprint/Cards/BP_CardParent.BP_CardParent_C|GetLeftValue (Variables|BP_CardSlot_C|GetCard%20Placed (Variables|Default|GetSlotRight))))
        (Rendering|Material|SetMaterial (Variables|BP_CardSlot_C|GetSlot _slotright) 0 "/Game/Blueprint/Cards/CardsTexture/BowmanTexture.BowmanTexture")
        (Variables|BP_CardSlot_C|SetIsOccupiedByPlayer _slotright true)
        (else
          (Variables|BP_CardSlot_C|SetIsOccupiedByBot _slotright true))))))