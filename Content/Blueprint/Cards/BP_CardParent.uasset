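; Base card actor for a Triad card game, taking its material and four side values from DT_Cards.
; Clicking makes it follow the cursor on Tick, and release runs SlotDetection to snap it onto a free overlapping slot.
; A valid slot reference triggers OnCardPlaced, smoke and a scaling flipbook whose timeline update notifies GM_Triad.
; Hover shows an outline, an info widget and side values that slide out by timeline.
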(event OnBeginCursorOver(Cube)
  (params (TouchedComponent :type Primitive%20Component%20Object%20Reference))
  ;[1 1 1] Ptit hover stylé
  (Rendering|Material|SetOverlayMaterial (Variables|Default|GetCube) "/Game/Blueprint/Cards/CardsTexture/CardOver.CardOver" :!class /Script/Engine.MeshComponent)
  (CallFunction|ShowStats)
  (bind _returnvalue (UserInterface|CreateWidget "/Game/Blueprint/Widgets/WB_CardInfos.WB_CardInfos_C"))
  (bind _output_get (Variables|Default|SetCardInfosRef _returnvalue))
  (UserInterface|Viewport|AddtoViewport _output_get 0)
  (bind _returnvalue_2 (Utilities|GetDataTableRow "/Game/Blueprint/Cards/DT_Cards.DT_Cards" (Variables|Default|GetRow%20Name))
    (:then
      (Appearance|SetBrushfromTexture (Variables|/Game/Blueprint/Widgets/WB_CardInfos.WB_CardInfos_C|GetCardIMG (Variables|Default|GetCardInfosRef)) (.cardtexture _returnvalue_2) false)
      (bind (_direction _movetoleft _movetoright _moveup _movedown) (Timeline|ShowStatsTL Play)
        (:Update
          (Transformation|SetRelativeLocation (Variables|Default|GetTextLeft) _movetoleft false false)
          (Transformation|SetRelativeLocation (Variables|Default|GetHoverRight) _movetoright false false)
          (Transformation|SetRelativeLocation (Variables|Default|GetHoverUp) _moveup false false)
          (Transformation|SetRelativeLocation (Variables|Default|GetHoverDown) _movedown false false))))))

(event OnEndCursorOver(Cube)
  (params (TouchedComponent :type Primitive%20Component%20Object%20Reference))
  ;[1 1 1] Ptit hover stylé
  (Rendering|Material|SetOverlayMaterial (Variables|Default|GetCube) 0 :!class /Script/Engine.MeshComponent)
  (Widget|RemovefromParent (Variables|Default|GetCardInfosRef))
  (bind (_direction _movetoleft _movetoright _moveup _movedown) (Timeline|ShowStatsTL Reverse)
    (:Update
      (Transformation|SetRelativeLocation (Variables|Default|GetTextLeft) _movetoleft false false)
      (Transformation|SetRelativeLocation (Variables|Default|GetHoverRight) _movetoright false false)
      (Transformation|SetRelativeLocation (Variables|Default|GetHoverUp) _moveup false false)
      (Transformation|SetRelativeLocation (Variables|Default|GetHoverDown) _movedown false false))))

(event EventBeginPlay
  ;[1 1 1] Recup l'info de quelle carte il doit être
  (CallFunction|GetandPrintDataInfos))

(event EventTick
  (params (DeltaSeconds :type Float%20%28single-precision%29))
  (bind _returnvalue (Game|GetPlayerController 0))
  (bind _hitresult (Game|Player|GetHitResultUnderCursorbyChannel _returnvalue "TraceTypeQuery1" true))
  ;[1 1 1] Grab la carte
  (if (Variables|Default|GetIsSelected?)
    (Transformation|SetActorLocation (Math|Vector|MakeVector (.x (.location _hitresult)) (.y (.location _hitresult)) 2e+01) false false)
    (Collision|SetCollisionResponsetoChannel (Variables|Default|GetCube) "ECC_Visibility" "ECR_Block")
    (else
      (Collision|SetCollisionEnabled (Variables|Default|GetCube) "QueryOnly"))))

(event EventActorOnReleased
  (params (ButtonReleased :type Key%20Structure :default "None"))
  (bind _smokeeffect (Variables|Default|GetSmokeEffect))
  (bind _sprite (Variables|Default|GetSprite))
  ;[1 1 1] Event quand la carte est relachée
  (bind _output_get (Variables|Default|SetIsSelected? false))
  (Development|PrintString (Utilities|String|Append "IsSelected?" (Utilities|String|ToString(Boolean) _output_get)))
  (Rendering|Material|SetOverlayMaterial (Variables|Default|GetCube) 0 :!class /Script/Engine.MeshComponent)
  ;;[0.3944 1 0.5036] Fonction pour se placer dans le slot
  (CallFunction|SlotDetection)
  (if (Utilities|IsValid (Variables|Default|GetAs%20BP%20Card%20Slot))
    ;;[0.3062 1 0.4374] Custom Event de BP_CardSlot pour lancer des actions
    (Default|OnCardPlaced (Variables|Default|GetAs%20BP%20Card%20Slot) self)
    (bind _returnvalue (Utilities|GetDataTableRow "/Game/Blueprint/Cards/DT_Cards.DT_Cards" (Variables|Default|GetRow%20Name))
      (:then
        (Utilities|FlowControl|Sequence
          (:then_0
            (Sprite|SetFlipbook _sprite (.spawner _returnvalue))
            (bind _scale (Timeline|ShowSpriteTL Play)
              (:Update
                (Transformation|SetWorldScale3D _sprite (Math|Vector|Lerp(Vector) "1.000000,1.000000,1.000000" "2.000000,2.000000,2.000000" _scale))
                (bind _asgm_triad (Utilities|Casting|CastToGM_Triad (Game|GetGameMode)))
                (Default|NotifyCardPlaced _asgm_triad))))
          (:then_1
            (Sprite|SetFlipbook _smokeeffect "/Game/Blueprint/Cards/CardsTexture/SmokeEffect/SmokeEffect.SmokeEffect")
            (Components|Timeline|SetLooping _smokeeffect false)))))))

(event MouseInput|EventActorOnClicked
  (params (ButtonPressed :type Key%20Structure :default "None"))
  ;[1 1 1] Event au grab de la carte
  (bind _output_get (Variables|Default|SetIsSelected? true))
  (Development|PrintString (Utilities|String|Append "IsSelected?" (Utilities|String|ToString(Boolean) _output_get)))
  (Rendering|Material|SetOverlayMaterial (Variables|Default|GetCube) "/Game/Blueprint/Cards/CardsTexture/CardOutliner.CardOutliner" :!class /Script/Engine.MeshComponent))

(fn ConstructionScript)

(fn GetandPrintDataInfos
  (bind _returnvalue (Utilities|GetDataTableRow "/Game/Blueprint/Cards/DT_Cards.DT_Cards" (Variables|Default|GetRow%20Name))
    (:then
      (Rendering|Material|SetMaterial (Variables|Default|GetCube) 0 (.cardimage _returnvalue))
      (Variables|Default|SetCardName (.cardname _returnvalue))
      (Variables|Default|SetTopValue (.topvalue _returnvalue))
      (Variables|Default|SetBottomValue (.bottomvalue _returnvalue))
      (Variables|Default|SetLeftValue (.leftvalue _returnvalue))
      (Variables|Default|SetRightValue (.rightvalue _returnvalue)))))

(fn SlotDetection
  (for _array_element (Collision|GetOverlappingActors "/Game/Blueprint/BP_CardSlot.BP_CardSlot_C" :!class /Script/Engine.Actor)
    (bind _asbp_card_slot (Utilities|Casting|CastToBP_CardSlot _array_element))
    (bind _output_get (Variables|Default|SetAs%20BP%20Card%20Slot _asbp_card_slot))
    (if (or (Variables|/Game/Blueprint/BP_CardSlot.BP_CardSlot_C|GetIsOccupiedByBot _output_get) (Variables|/Game/Blueprint/BP_CardSlot.BP_CardSlot_C|GetIsOccupiedByPlayer _asbp_card_slot))
      (Variables|Default|SetIsLocked false)
      (Development|PrintString "Je ne peux pas me placer il y a déjà une carte" true true "(R=0.692244,G=0.000000,B=1.000000,A=1.000000)")
      (else
        (Transformation|SetActorLocation (Math|Vector|MakeVector (.x (Transformation|GetActorLocation _asbp_card_slot)) (.y (Transformation|GetActorLocation _asbp_card_slot)) 1e+01) false false)
        (Variables|Default|SetIsLocked true)
        (bind _output_get_2 (Variables|Default|SetCardOwner "NewEnumerator0"))
        (Development|PrintString (Utilities|String|EnumtoString _output_get_2) true true "(R=1.000000,G=0.396698,B=0.133661,A=1.000000)")))))

(fn ShowStats
  (Rendering|Components|TextRender|SetText (Variables|Default|GetTextUp) (Utilities|Text|ToText(Integer) (Variables|Default|GetTopValue)))
  (Rendering|Components|TextRender|SetText (Variables|Default|GetTextDown) (Utilities|Text|ToText(Integer) (Variables|Default|GetBottomValue)))
  (Rendering|Components|TextRender|SetText (Variables|Default|GetTextLeft) (Utilities|Text|ToText(Integer) (Variables|Default|GetLeftValue)))
  (Rendering|Components|TextRender|SetText (Variables|Default|GetTextRight) (Utilities|Text|ToText(Integer) (Variables|Default|GetRightValue)))
  (Rendering|SetVisibility (Variables|Default|GetTextUp) true false))

(fn HideStats
  (Rendering|SetVisibility (Variables|Default|GetTextUp) false false))