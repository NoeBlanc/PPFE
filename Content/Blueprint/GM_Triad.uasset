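; GM_Triad, apparently the game mode of a card game, detects when the match is over and decides the winner.
; NotifyCardPlaced counts locked BP_CardParent actors and calls FinishGame once every card in the level is locked.
; FinishGame tallies cards as Player or Bot and announces the side with more through debug print strings, with ties going to the Bot.
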(fn ConstructionScript)

(fn NotifyCardPlaced
  (bind _outactors (Actor|GetAllActorsOfClass "/Game/Blueprint/Cards/BP_CardParent.BP_CardParent_C"))
  (for _array_element _outactors
    (if (not (not (Variables|/Game/Blueprint/Cards/BP_CardParent.BP_CardParent_C|GetIsLocked _array_element)))
      (Math|Integer|IncrementInt (LocalVariables|GetLocalCardNb))))
  (if (== (Utilities|Array|Length _outactors) (LocalVariables|GetLocalCardNb))
    (Development|PrintString "FIN DE PARTIE" true true "(R=0.007468,G=0.473958,B=0.000000,A=1.000000)")
    (CallFunction|FinishGame)))

(fn FinishGame
  (bind _outactors (Actor|GetAllActorsOfClass "/Game/Blueprint/Cards/BP_CardParent.BP_CardParent_C"))
  (for _array_element _outactors
    (switch Utilities|FlowControl|Switch|SwitchonCardOwner "NewEnumerator0"
      (:NewEnumerator0
        (Math|Integer|IncrementInt (LocalVariables|GetPlayerCount)))
      (:NewEnumerator1
        (Math|Integer|IncrementInt (LocalVariables|GetBotCount)))))
  (if (> (LocalVariables|GetPlayerCount) (LocalVariables|GetBotCount))
    (Development|PrintString "Player gagne")
    (else
      (Development|PrintString "Bot gagne"))))